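; BP_InteractionBlueprint handles the interaction that throws a bomb at a hole that needs one.
; HandleInteraction stores the given hole and spawn component, then spawns a BP_Bomb at that component if the hole is valid and needs a bomb.
; It pushes the bomb's mesh horizontally toward the hole with a force that grows with distance squared, then passes the bomb to the hole's OnBombPlaced.
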(fn `HandleInteraction`
  (params (Hole :type "/Game/VehicleAdvBP/Blueprints/Holes/BP_Hole Object Reference") (BombSpawnPlace :type "InstancedStaticMeshComponent Object Reference"))
  (locals (OverlappingHole :type "/Game/VehicleAdvBP/Blueprints/Holes/BP_Hole Object Reference") (SpawnPlace :type "InstancedStaticMeshComponent Object Reference"))
  (bind _overlappinghole (`local.OverlappingHole`))
  (bind _returnvalue_location (`KismetMathLibrary.BreakTransform` (`SceneComponent.K2_GetComponentToWorld` (`local.BombSpawnPlace`))))
  (bind _returnvalue_location_2 (`KismetMathLibrary.BreakTransform` (`self.GetTransform` (`local.OverlappingHole`))))
  (bind (_returnvalue_x _returnvalue_y) (`KismetMathLibrary.BreakVector` (- _returnvalue_location_2 _returnvalue_location)))
  (bind _returnvalue (`KismetMathLibrary.MakeVector` _returnvalue_x _returnvalue_y))
  (set `local.OverlappingHole` Hole)
  (set `local.SpawnPlace` BombSpawnPlace)
  (if (and (`KismetSystemLibrary.IsValid` _overlappinghole) (`/Game/VehicleAdvBP/Blueprints/Holes/BP_Hole.NeedsBomb` _overlappinghole))
    ;[1 1 1] Spawn bomb
    (bind _returnvalue_2 (`|SpawnActorFromClass` "/Game/VehicleAdvBP/Blueprints/Bomb/BP_Bomb.BP_Bomb_C" (`SceneComponent.K2_GetComponentToWorld` (`local.BombSpawnPlace`)) "Undefined" "OverrideRootScale" null null))
    (`PrimitiveComponent.AddForce` (`/Game/VehicleAdvBP/Blueprints/Bomb/BP_Bomb.Mesh` _returnvalue_2) (* _returnvalue (* 2 (`KismetMathLibrary.VSize` _returnvalue))) "None" false)
    (`/Game/VehicleAdvBP/Blueprints/Holes/BP_Hole.OnBombPlaced` (`local.OverlappingHole`) _returnvalue_2)))

(fn `UserConstructionScript`)