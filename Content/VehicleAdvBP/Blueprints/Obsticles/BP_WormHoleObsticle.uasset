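; BP_WormHoleObsticle is a hazard actor that damages the player vehicle on contact and destroys itself.
; When its Box overlaps a VehicleBlueprint, it subtracts Damage from that vehicle's WormHollHealth, then spawns an explosion emitter and sound at its own location.
; If that health is no longer above zero, it calls Death on the vehicle.
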(event `self.Box.OnComponentBeginOverlap`
  (params (OverlappedComponent :type "PrimitiveComponent Object Reference") (OtherActor :type "Actor Object Reference") (OtherComp :type "PrimitiveComponent Object Reference") (OtherBodyIndex :type Integer) (bFromSweep :type Boolean) (SweepResult :type "HitResult Structure (by ref)"))
  (bind _returnvalue (`self.K2_GetActorLocation` self))
  (bind _asvehicle_blueprint (cast `/Game/VehicleAdvBP/Blueprints/VehicleBlueprint` OtherActor))
  (bind _output_get (set `/Game/VehicleAdvBP/Blueprints/VehicleBlueprint.WormHollHealth` (- (`/Game/VehicleAdvBP/Blueprints/VehicleBlueprint.WormHollHealth` _asvehicle_blueprint) (`self.Damage`)) _asvehicle_blueprint))
  (`GameplayStatics.SpawnEmitterAtLocation` "/Game/Materials/P_Explosion.P_Explosion" _returnvalue)
  (`GameplayStatics.PlaySoundAtLocation` "/Game/VehicleAdv/Sound/Explosion1.Explosion1" _returnvalue (struct) 1.0 1.0 0.0 null null null)
  (`self.K2_DestroyActor`)
  (if (not (> _output_get 0.0))
    (`/Game/VehicleAdvBP/Blueprints/VehicleBlueprint.Death` _asvehicle_blueprint)))

(fn `UserConstructionScript`)