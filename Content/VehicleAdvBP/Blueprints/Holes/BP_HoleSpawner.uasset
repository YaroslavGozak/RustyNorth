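; BP_HoleSpawner spawns BP_Hole actors one at a time at placeholder locations, up to a set count.
; On BeginPlay it gathers BP_HolePlace markers and the BP_HolePlaceLast marker, then spawns the first hole.
; Each SpawnNextHole call picks a random marker, then removes and destroys it to prevent reuse.
; The final hole in the count spawns at the dedicated last marker, flagged IsLast.
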(event `self.ReceiveBeginPlay`
  ;[1 1 1] Initialize hole placeholders
  (bind _outactors (`GameplayStatics.GetAllActorsOfClass` "/Game/VehicleAdvBP/Blueprints/Holes/BP_HolePlace.BP_HolePlace_C"))
  (set `self.HolePlaces` _outactors)
  ;[1 1 1] Get last hole placeholder
  (bind _returnvalue (`GameplayStatics.GetActorOfClass` "/Game/VehicleAdvBP/Blueprints/Holes/BP_HolePlaceLast.BP_HolePlaceLast_C"))
  (set `self.LastHole` _returnvalue)
  ;[1 1 1] Spawn first hole
  (`self.SpawnNextHole`))

(event `SpawnNextHole`
  (if (> (`self.HolesCount`) (`self.HolesSpawned`))
    (if (== (- (`self.HolesCount`) 1) (`self.HolesSpawned`))
      (`self.SpawnLastHole`)
      (else
        (`self.TrySpawnHole`)))
    (`KismetSystemLibrary.PrintString` "Hole spawned")
    (else
      (`KismetSystemLibrary.PrintString` "Already spawned enough holes"))))

(fn `SpawnHole`
  (params (Transform :type "Transform Structure") (IsLast :type Boolean))
  (`|SpawnActorFromClass` "/Game/VehicleAdvBP/Blueprints/Holes/BP_Hole.BP_Hole_C" Transform "Undefined" "OverrideRootScale" null IsLast null)
  ;[1 1 1] Increment spawned holes
  (bind _result (`/Engine/EditorBlueprintResources/StandardMacros.IncrementInt` (`self.HolesSpawned`))
    (:`  `
      (set `self.HolesSpawned` _result))))

(fn `SpawnLastHole`
  (`self.SpawnHole` (`self.GetTransform` (`self.LastHole`)) true))

(fn `TrySpawnHole`
  (locals (MinIndex :type Integer :default 1000))
  (if (> (`KismetArrayLibrary.Array_Length` (`self.HolePlaces`)) 0)
    ;[1 1 1] Get random hole
    (bind _output_get (set `self.HolePlaceToSpawn` (`|GetArrayItem` (`self.HolePlaces`) (`KismetMathLibrary.RandomIntegerInRange` 0 (- (`KismetArrayLibrary.Array_Length` (`self.HolePlaces`)) 1)))))
    (`self.SpawnHole` (`self.GetTransform` _output_get))
    ;[1 1 1] Remove hole place from array and also delete it from level
    (bind _returnvalue (`KismetArrayLibrary.Array_RemoveItem` (`self.HolePlaces`) (`self.HolePlaceToSpawn`)))
    (if (not _returnvalue)
      (`KismetSystemLibrary.PrintString` "WARNING: Hole could not be removed from array" true true (struct :`R` 1.0 :`G` 0.688825 :`A` 1.0)))
    ;;[1 1 1] Try to destroy this hole spawn place
    (`self.K2_DestroyActor` (`self.HolePlaceToSpawn`))
    (else
      (`KismetSystemLibrary.PrintString` "No holes to spawn"))))

(fn `UserConstructionScript`)