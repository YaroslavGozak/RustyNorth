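; BP_HoleNoCollision is a hole actor that can receive a bomb and later switch to a destroyed look.
; It finds the BP_HoleSpawner on BeginPlay; when a bomb is placed it stores it, resets its tags and asks the spawner to spawn the next hole.
; NeedsBomb reports whether a bomb is still missing, and DestroyHole swaps the intact mesh for the destroyed one by toggling visibility.
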(event `self.ReceiveBeginPlay`
  (bind _returnvalue (`GameplayStatics.GetActorOfClass` "/Game/VehicleAdvBP/Blueprints/Holes/BP_HoleSpawner.BP_HoleSpawner_C"))
  (set `self.HoleSpawner` _returnvalue))

(event `OnBombPlaced`
  (params (SetBomb :type "/Game/VehicleAdvBP/Blueprints/Bomb/BP_Bomb Object Reference"))
  (set `self.Bomb` SetBomb)
  (`KismetSystemLibrary.PrintString` "Bomb set up")
  (set `self.Tags` (`|MakeArray` "None" :!type "Name"))
  (`/Game/VehicleAdvBP/Blueprints/Holes/BP_HoleSpawner.SpawnNextHole` (`self.HoleSpawner`)))

(event `DestroyHole`
  (`SceneComponent.SetVisibility` (`self.HoleStaticMesh`) false true)
  (`SceneComponent.SetVisibility` (`self.HoleDestroyedStaticMesh`) true true))

(fn `NeedsBomb`
  (returns (NeedsBomb :type Boolean))
  (return (not (`KismetSystemLibrary.IsValid` (`self.Bomb`)))))

(fn `UserConstructionScript`)