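; BP_Hole is a hole actor that takes a bomb and can switch to a destroyed look.
; On BeginPlay it caches the level's BP_HoleSpawner, and NeedsBomb reports whether it still lacks a valid bomb.
; OnBombPlaced attaches the given bomb to the hole, stores it and asks the spawner for the next hole.
; DestroyHole swaps visibility from the intact mesh to the destroyed mesh.
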(event `self.ReceiveBeginPlay`
  (bind _returnvalue (`GameplayStatics.GetActorOfClass` "/Game/VehicleAdvBP/Blueprints/Holes/BP_HoleSpawner.BP_HoleSpawner_C"))
  (set `self.HoleSpawner` _returnvalue))

(event `OnBombPlaced`
  (params (SetBomb :type "/Game/VehicleAdvBP/Blueprints/Bomb/BP_Bomb Object Reference"))
  (`/Game/VehicleAdvBP/Blueprints/Bomb/BP_Bomb.AttachToHole` SetBomb self)
  (set `self.Bomb` SetBomb)
  (`KismetSystemLibrary.PrintString` "Bomb set up")
  (`/Game/VehicleAdvBP/Blueprints/Holes/BP_HoleSpawner.SpawnNextHole` (`self.HoleSpawner`)))

(event `DestroyHole`
  (`SceneComponent.SetVisibility` (`self.HoleStaticMesh`) false true)
  (`SceneComponent.SetVisibility` (`self.HoleDestroyedStaticMesh`) true true))

(fn `NeedsBomb`
  (returns (NeedsBomb :type Boolean))
  (return (not (`KismetSystemLibrary.IsValid` (`self.Bomb`)))))

(fn `UserConstructionScript`)