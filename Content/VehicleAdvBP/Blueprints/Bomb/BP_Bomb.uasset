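; Bomb actor that flies from its spawn point to a socket on its Hole, then destroys the hole and itself when a countdown expires.
; On BeginPlay it starts a looping one-second timer and caches the spawn and socket locations.
; The Movement timeline adds a curve offset to a blend along that direction to set its position.
; The timer decrements and prints Seconds, calling Kaboom at zero.
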(event `self.ReceiveBeginPlay`
  (`self.AttachToHole`)
  (`self.GetTargetLocation`)
  (`self.GetSpawnLocation`)
  (set `self.MoveDirection` (- (`self.TargetLocation`) (`self.SpawnLocation`)))
  (bind (_direction _curve _blend) (`Timeline|Movement` :!via `PlayFromStart`)
    (:`Update`
      (`SceneComponent.K2_SetWorldLocation` (`self.DefaultSceneRoot`) (+ (`self.SpawnLocation`) (+ _curve (* (`self.MoveDirection`) _blend))) false false))))

(event `AttachToHole`
  (bind _returnvalue (`KismetSystemLibrary.K2_SetTimerDelegate` (delegate `CountDown`) 1.0 true))
  (set `self.Timer` _returnvalue))

(event `CountDown`
  (bind _result (`/Engine/EditorBlueprintResources/StandardMacros.DecrementInt` (`self.Seconds`))
    (:`  `
      (bind _output_get (set `self.Seconds` _result))
      (`KismetSystemLibrary.PrintString` (`KismetStringLibrary.Conv_IntToString` _output_get))
      (if (== _output_get 0)
        (`self.Kaboom`)))))

(event `Kaboom`
  (`KismetSystemLibrary.PrintString` "Kaboom")
  (`KismetSystemLibrary.K2_InvalidateTimerHandle` (`self.Timer`))
  (`/Game/VehicleAdvBP/Blueprints/Holes/BP_Hole.DestroyHole` (`self.Hole`))
  (`self.K2_DestroyActor`))

(fn `GetSpawnLocation`
  (set `self.SpawnLocation` (`SceneComponent.K2_GetComponentLocation` (`self.DefaultSceneRoot`))))

(fn `GetTargetLocation`
  (set `self.TargetLocation` (`SceneComponent.GetSocketLocation` (`/Game/VehicleAdvBP/Blueprints/Holes/BP_Hole.HoleStaticMesh` (`self.Hole`)) (`self.BombPlace`))))

(fn `UserConstructionScript`)